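; Player controller Blueprint for MakeMyHappy that evaluates a pair of selected CircleEvent buttons.
; Its Choose event acts only when ChoosenButtons holds exactly two entries, comparing their hero and level IDs.
; When both IDs differ, it sets each button's background to white; other pairs are left untouched, and the array is not cleared here.
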(event Custom|Choose
  (bind _choosenbuttons (Variables|Default|GetChoosenButtons))
  (if (== (Utilities|Array|Length (Variables|Default|GetChoosenButtons)) 2)
    (bind _ascircle_event (Utilities|Casting|CastToCircleEvent (Utilities|Array|Get(acopy) _choosenbuttons)))
    (bind _ascircle_event_2 (Utilities|Casting|CastToCircleEvent (Utilities|Array|Get(acopy) _choosenbuttons 1)))
    (if (and (!= (Variables|/Game/MakeMyHappy/Widgets/CircleEvent.CircleEvent_C|GetidHero _ascircle_event_2) (Variables|/Game/MakeMyHappy/Widgets/CircleEvent.CircleEvent_C|GetidHero _ascircle_event)) (!= (Variables|/Game/MakeMyHappy/Widgets/CircleEvent.CircleEvent_C|GetidLevel _ascircle_event_2) (Variables|/Game/MakeMyHappy/Widgets/CircleEvent.CircleEvent_C|GetidLevel _ascircle_event)))
      (for _array_element (Variables|Default|GetChoosenButtons)
        (bind _ascircle_event_3 (Utilities|Casting|CastToCircleEvent _array_element))
        (Class|Button|SetBackgroundColor (Variables|/Game/MakeMyHappy/Widgets/CircleEvent.CircleEvent_C|GetButton_65 _ascircle_event_3) "(R=1.000000,G=1.000000,B=1.000000,A=1.000000)")))))

(event EventBeginPlay)

(event EventTick
  (params (DeltaSeconds :type Float%20%28single-precision%29)))

(fn ConstructionScript)